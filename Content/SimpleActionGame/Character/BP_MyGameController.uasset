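; Player controller for the simple action game that sets up the local player's HUD and a debug save key.
; On BeginPlay, a local controller creates the game-time, simple UI and player-health widgets, adds them to the viewport and switches input to game-only mode.
; Pressing L casts the game mode to MGameModeBase, calls WriteSaveGame and prints a confirmation.
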(event EventBeginPlay
  (if (Pawn|IsLocalController)
    (bind _returnvalue (UserInterface|CreateWidget "/Game/SimpleActionGame/UI/GameTime_UI.GameTime_UI_C"))
    (UserInterface|Viewport|AddtoViewport _returnvalue 0)
    (bind _returnvalue_2 (UserInterface|CreateWidget "/Game/SimpleActionGame/UI/SimpleUI.SimpleUI_C"))
    (UserInterface|Viewport|AddtoViewport _returnvalue_2 0)
    (bind _returnvalue_3 (UserInterface|CreateWidget "/Game/SimpleActionGame/UI/PlayerHealth_UI.PlayerHealth_UI_C"))
    (UserInterface|Viewport|AddtoViewport _returnvalue_3 0)
    (Input|SetInputModeGameOnly self)))

(event EventTick
  (params (DeltaSeconds :type Float%20%28single-precision%29)))

(event Input|KeyboardEvents|L
  (params (Key :type Key%20Structure :default "None"))
  (:Pressed
    (bind _asmgame_mode_base (Utilities|Casting|CastToMGameModeBase (Game|GetGameMode)))
    (Class|MGameModeBase|WriteSaveGame _asmgame_mode_base)
    (Development|PrintString "SaveGame")))

(fn ConstructionScript)