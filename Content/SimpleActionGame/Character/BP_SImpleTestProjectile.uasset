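; Test actor that repeatedly fires BP_PrimaryAttack_AI projectiles, acting as a simple turret.
; BeginPlay starts a looping two-second timer that spawns the attack at the actor's location and rotation.
; Tick turns the Arrow component to face the player pawn.
; After each spawn, it checks the player's MAttributeComponent and clears the timer once the player is no longer alive.
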(event Custom|particle
  (Game|SpawnActorfromClass "/Game/SimpleActionGame/Character/Attack/BP_PrimaryAttack_AI.BP_PrimaryAttack_AI_C" (Math|Transform|MakeTransform (Transformation|GetActorLocation) (Transformation|GetActorRotation)) "Undefined" 0 0)
  (if (not (Class|MAttributeComponent|IsAlive (Actor|GetComponentbyClass (Game|Player|GetPlayerPawn 0) "/Script/ActionRogue.MAttributeComponent")))
    (Utilities|Time|ClearandInvalidateTimerbyHandle (Variables|Default|GetTimerHandle))))

(event EventBeginPlay
  (bind _returnvalue (Utilities|Time|SetTimerbyEvent (delegate Custom|particle) 2.0 true))
  (Variables|Default|SetTimerHandle _returnvalue))

(event Collision|EventActorBeginOverlap
  (params (OtherActor :type Actor%20Object%20Reference)))

(event EventTick
  (params (DeltaSeconds :type Float%20%28single-precision%29))
  (Transformation|SetWorldRotation (Variables|Default|GetArrow) (Math|Rotator|FindLookatRotation (Transformation|GetActorLocation) (Transformation|GetActorLocation (Game|Player|GetPlayerPawn 0))) false false))

(fn ConstructionScript)